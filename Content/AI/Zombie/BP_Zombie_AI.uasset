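; AI controller for zombies that runs the BT_Zombie behavior tree and tracks whether the player is seen.
; On BeginPlay it registers itself on the pawn and seeds the Blackboard with spawn location, zombie roam and attack tuning, and the player's PointsNearPlayer.
; Pawns flagged BadPerception switch sight to a second perception component.
; Both components share one handler that sets or clears focus, updates CanSeePlayer and notifies the pawn for debugging.
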(event `self.ReceiveBeginPlay`
  (bind _blackboard (`self.Blackboard`))
  (`self.RunBehaviorTree` "/Game/AI/Zombie/BT_Zombie.BT_Zombie")
  (bind _asbp_zombie (cast `/Game/AI/Zombie/BP_Zombie` (`self.K2_GetPawn`)))
  (bind _output_get (set `self.MyPawn` _asbp_zombie))
  (set `/Game/AI/Zombie/BP_Zombie.MyAIController` self _output_get)
  (if (`/Game/AI/Zombie/BP_Zombie.BadPerception` _output_get)
    (`AIPerceptionComponent.SetSenseEnabled` (`self.AIPerception`) "/Script/AIModule.AISense_Sight" false)
    (`AIPerceptionComponent.SetSenseEnabled` (`self.AIPerception_Bad`) "/Script/AIModule.AISense_Sight" true))
  (`BlackboardComponent.SetValueAsVector` _blackboard "SpawnLocation" (`self.K2_GetActorLocation` _output_get))
  (`BlackboardComponent.SetValueAsFloat` _blackboard "RoamRadius" (`/Game/AI/Zombie/BP_Zombie.RoamRadius` _output_get))
  (`BlackboardComponent.SetValueAsFloat` _blackboard "RoamWaitTIme" (`/Game/AI/Zombie/BP_Zombie.RoamWaitTime` _output_get))
  (`BlackboardComponent.SetValueAsFloat` _blackboard "LostWaitTIme" (`/Game/AI/Zombie/BP_Zombie.LostWaitTime` _output_get))
  (`BlackboardComponent.SetValueAsFloat` _blackboard "AttackCooldown" (`/Game/AI/Zombie/BP_Zombie.AttackCooldown` _output_get))
  (`BlackboardComponent.SetValueAsFloat` _blackboard "AttackStartDistance" (`/Game/AI/Zombie/BP_Zombie.AttackStartDistance` _output_get))
  (bind _asthird_person_character (cast `/Game/ThirdPersonBP/Blueprints/ThirdPersonCharacter` (`GameplayStatics.GetPlayerCharacter` 0)))
  (`BlackboardComponent.SetValueAsInt` _blackboard "PointsNearPlayer" (`/Game/ThirdPersonBP/Blueprints/ThirdPersonCharacter.PointsNearPlayer` _asthird_person_character)))

(event `self.AIPerception.OnTargetPerceptionUpdated`
  (params (Actor :type "Actor Object Reference") (Stimulus :type "AIStimulus Structure"))
  ;[0 0.1 0.5] Perception Sight
  (`self.OnTargetPerceptionUpdated` Actor Stimulus))

(event `OnTargetPerceptionUpdated`
  (params (Actor :type "Actor Object Reference") (Stimulus :type "AIStimulus Structure"))
  (bind (_age _expirationage _strength _stimuluslocation _receiverlocation _tag _bsuccessfullysensed) (break `AIStimulus` Stimulus))
  ;[0 0.1 0.5] Perception Sight
  (bind _asthird_person_character (cast `/Game/ThirdPersonBP/Blueprints/ThirdPersonCharacter` Actor))
  (if _bsuccessfullysensed
    (`self.K2_SetFocus` _asthird_person_character)
    (else
      (`self.K2_SetFocus` null)))
  (`BlackboardComponent.SetValueAsBool` (`self.Blackboard`) "CanSeePlayer" _bsuccessfullysensed) ; Отправляем "видно/не видно" в BB
  (`/Game/AI/Zombie/BP_Zombie.SeePlayer` (`self.MyPawn`) _bsuccessfullysensed) ; Для дебага
)

(event `self.AIPerception_Bad.OnTargetPerceptionUpdated`
  (params (Actor :type "Actor Object Reference") (Stimulus :type "AIStimulus Structure"))
  ;[0 0.1 0.5] Perception Sight
  (`self.OnTargetPerceptionUpdated` Actor Stimulus))

(fn `UserConstructionScript`)