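; Zombie AI character that switches between roam and chase speeds and melee-attacks through its AnimBP, with perception ranges set at BeginPlay.
; Queue and attack approval events update its number and Blackboard flags for the AI controller.
; Overlapping the player disables avoidance and movement-oriented rotation to prevent shoving, while AIPlaceOccupier stays pinned at the attack start position during engagement.
; A toggleable debug view shows state-colored text and a sight cone.
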(event `self.ReceiveBeginPlay`
  (set `self.MyName` (`KismetSystemLibrary.GetDisplayName` self))
  (`SceneComponent.SetVisibility` (`self.DebugText`) false false)
  (if (`self.BadPerception`)
    (set `self.SightSpotRadius` 750.0)
    (set `self.SightLoseRadius` 1000.0)
    (else
      (set `self.SightSpotRadius` 1500.0)
      (set `self.SightLoseRadius` 2000.0)))
  (`/Game/AI/Zombie/Zombie_Interface.ReturnToSpawn` true)
  (bind _aszombie_anim_bp (cast `/Game/Assets/zombie_character/Animations/zombie_AnimBP` (`SkeletalMeshComponent.GetAnimInstance` (`self.Mesh`))))
  (bind _output_get (set `self.MyAnimBP` _aszombie_anim_bp))
  (set `/Game/Assets/zombie_character/Animations/zombie_AnimBP.CharRef` self _output_get))

(event `/Game/AI/Zombie/Zombie_Interface.SetChasing`
  (params (IsChasing :type Boolean))
  (bind _charactermovement (`self.CharacterMovement`))
  (if IsChasing
    (set `CharacterMovementComponent.MaxWalkSpeed` (* 325.0 (`self.ChaseSpeedModifier`)) _charactermovement)
    (else
      (set `CharacterMovementComponent.MaxWalkSpeed` (* 65.0 (`self.RoamSpeedModifier`)) _charactermovement))))

(event `/Game/AI/Zombie/Zombie_Interface.AttackApproved`
  (`BlackboardComponent.SetValueAsBool` (`AIController.Blackboard` (`self.MyAIController`)) "AttackApproved" true)
  (`self.RefreshDebugText` false))

(event `/Game/AI/Zombie/Zombie_Interface.SetQueueNumber`
  (params (Number :type Integer))
  (set `self.MyQueueNumber` Number)
  (`self.RefreshDebugText` true))

(event `/Game/AI/Zombie/Zombie_Interface.RefreshQueueNumber`
  (params (InQueue :type Boolean))
  (`self.RefreshDebugText` InQueue))

(event `/Game/AI/Zombie/Zombie_Interface.MeleeAttack`
  (params (Status :type Boolean))
  (bind _output_get (set `self.IsAttacking` Status))
  (if _output_get
    (`/Game/Assets/zombie_character/Animations/zombie_AnimBP.MeleeAttackAnim` (`self.MyAnimBP`) (`self.Mesh`) (`self.AttackSpeed`))
    (else
      (`BlackboardComponent.SetValueAsBool` (`AIController.Blackboard` (`self.MyAIController`)) "IsAttacking" false)
      (if (not (`self.IsOverlapping`))
        (set `CharacterMovementComponent.bOrientRotationToMovement` true (`self.CharacterMovement`)) ; Вне атаки
      ))))

(event `self.OverlapCollision.OnComponentBeginOverlap`
  (params (OverlappedComponent :type "PrimitiveComponent Object Reference") (OtherActor :type "Actor Object Reference") (OtherComp :type "PrimitiveComponent Object Reference") (OtherBodyIndex :type Integer) (bFromSweep :type Boolean) (SweepResult :type "HitResult Structure (by ref)"))
  ;[0.5 0.5 0.5] Чтобы в ближнем бою не толкался и отходил задом
  (cast `/Game/ThirdPersonBP/Blueprints/ThirdPersonCharacter` OtherActor)
  (`CharacterMovementComponent.SetAvoidanceEnabled` (`self.CharacterMovement`) false)
  (set `self.IsOverlapping` true)
  (set `CharacterMovementComponent.bOrientRotationToMovement` false (`self.CharacterMovement`)))

(event `self.OverlapCollision.OnComponentEndOverlap`
  (params (OverlappedComponent :type "PrimitiveComponent Object Reference") (OtherActor :type "Actor Object Reference") (OtherComp :type "PrimitiveComponent Object Reference") (OtherBodyIndex :type Integer))
  (bind _charactermovement (`self.CharacterMovement`))
  ;[0.5 0.5 0.5] Чтобы в ближнем бою не толкался и отходил задом
  (cast `/Game/ThirdPersonBP/Blueprints/ThirdPersonCharacter` OtherActor)
  (`CharacterMovementComponent.SetAvoidanceEnabled` _charactermovement true)
  (set `self.IsOverlapping` false)
  (if (and (not (`self.IsAttacking`)) (not (`CharacterMovementComponent.bOrientRotationToMovement` _charactermovement)))
    (set `CharacterMovementComponent.bOrientRotationToMovement` true (`self.CharacterMovement`))))

(event `/Game/AI/Zombie/Zombie_Interface.OccupyPlace`
  (params (PlaceVector :type "Vector Structure") (IsFinished :type Boolean))
  (bind _output_get (set `self.HasEngaged` (not IsFinished)))
  (if _output_get
    (set `self.AttackStartPosition` PlaceVector)
    (else
      (`SceneComponent.K2_SetRelativeLocation` (`self.AIPlaceOccupier`) (`KismetMathLibrary.Vector_Zero`) false true) ; Вернуть Occupier обратно
    )))

(event `self.ReceiveTick`
  (params (DeltaSeconds :type "Float (single-precision)"))
  (if (`self.HasEngaged`)
    (`SceneComponent.K2_SetWorldLocation` (`self.AIPlaceOccupier`) (`self.AttackStartPosition`) false true) ; Держать Occupier на стартовой точке
  )
  (if (`self.IsDebug`)
    (`self.DebugTick`)))

(event `DebugHotkey`
  ;[0 0.5 0.5] Debug
  (bind _output_get (set `self.IsDebug` (not (`self.IsDebug`))))
  (`SceneComponent.SetVisibility` (`self.DebugText`) _output_get false)
  (`BlackboardComponent.SetValueAsBool` (`AIController.Blackboard` (`self.MyAIController`)) "IsDebug" _output_get))

(event `DebugTick`
  (bind _returnvalue (`self.K2_GetActorLocation`))
  ;[0 0.5 0.5] Debug
  (`SceneComponent.K2_SetWorldRotation` (`self.DebugText`) (`KismetMathLibrary.FindLookAtRotation` _returnvalue (`self.K2_GetActorLocation` (`GameplayStatics.GetPlayerCameraManager` 0))) false false)
  (`KismetSystemLibrary.DrawDebugConeInDegrees` _returnvalue (`KismetMathLibrary.GetForwardVector` (`self.K2_GetActorRotation` (`self.MyAIController`))) (`self.CurrentSight`) 75.0 75.0 12 (`self.CurrentDebugColor`)))

(event `SeePlayer`
  (params (CanSeePlayer :type Boolean))
  (bind _debugtext (`self.DebugText`))
  (bind _debugtext_2 (`self.DebugText`))
  ;[0 0.5 0.5] Debug
  (if CanSeePlayer
    (`TextRenderComponent.K2_SetText` _debugtext_2 (`self.SetDebugText` "Aggressive"))
    (bind _output_get (set `self.CurrentDebugColor` (`KismetMathLibrary.LinearColor_Red`)))
    (`TextRenderComponent.SetTextRenderColor` _debugtext (`KismetMathLibrary.Conv_LinearColorToColor` _output_get))
    (set `self.CurrentSight` (`self.SightLoseRadius`))
    (else
      (`TextRenderComponent.K2_SetText` _debugtext_2 (`self.SetDebugText` "Lost"))
      (bind _output_get_2 (set `self.CurrentDebugColor` (`KismetMathLibrary.LinearColor_Gray`)))
      (`TextRenderComponent.SetTextRenderColor` _debugtext (`KismetMathLibrary.Conv_LinearColorToColor` _output_get_2))
      (set `self.CurrentSight` (`self.SightSpotRadius`)))))

(event `/Game/AI/Zombie/Zombie_Interface.ReturnToSpawn`
  (params (IsFinished :type Boolean))
  (bind _debugtext (`self.DebugText`))
  (bind _debugtext_2 (`self.DebugText`))
  ;[0 0.5 0.5] Debug
  (if IsFinished
    (`TextRenderComponent.K2_SetText` _debugtext (`self.SetDebugText` "Calm"))
    (bind _output_get (set `self.CurrentDebugColor` (`KismetMathLibrary.LinearColor_Green`)))
    (`TextRenderComponent.SetTextRenderColor` _debugtext_2 (`KismetMathLibrary.Conv_LinearColorToColor` _output_get))
    (else
      (`TextRenderComponent.K2_SetText` _debugtext (`self.SetDebugText` "Returning"))
      (bind _output_get_2 (set `self.CurrentDebugColor` (`KismetMathLibrary.LinearColor_Blue`)))
      (`TextRenderComponent.SetTextRenderColor` _debugtext_2 (`KismetMathLibrary.Conv_LinearColorToColor` _output_get_2))))
  (set `self.CurrentSight` (`self.SightSpotRadius`)))

(fn `UserConstructionScript`)